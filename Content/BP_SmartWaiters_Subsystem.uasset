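; BP_SmartWaiters_Subsystem moves items from provider stations to request stations that have run out of their requested item.
; On the authority, a looping timer scans all stations and creates an order wherever a provider's count of that item meets DeliveryThreshold.
; Orders instantly teleport the provider's slot 0 stack without checking its type.
; The provider loop keeps going after an order, so one request can draw from several providers per tick.
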(event Custom|Waiters_Tick
  (bind _outactors (Actor|GetAllActorsOfClass "/SmartWaiters/Buildings/Stations/BP_RequestStation.BP_RequestStation_C"))
  (if (> (Utilities|Array|Length _outactors) 0)
    (bind _outactors_2 (Actor|GetAllActorsOfClass "/SmartWaiters/Buildings/Stations/BP_ProviderStation.BP_ProviderStation_C"))
    (for _array_element _outactors
      (if (.HasNeed (CallFunction|GetRequestItems _array_element))
        (for _array_element_2 _outactors_2
          (if (>= (CallFunction|GetAvailableItems _array_element_2 (.NeededItemType (CallFunction|GetRequestItems _array_element))) (Variables|Default|GetDeliveryThreshold))
            (CallFunction|CreateOrder _array_element_2 _array_element (.NeededItemType (CallFunction|GetRequestItems _array_element)))))))))

(event EventBeginPlay
  (Networking|SwitchHasAuthority
    (:Authority
      (Utilities|Time|SetTimerbyEvent (delegate Custom|Waiters_Tick) (Variables|Default|GetTickSpeed) true))))

(fn ConstructionScript)

(fn GetRequestItems
  (params (RequestStation :type BP%20Request%20Station%20Object%20Reference))
  (bind _itemtype (LocalVariables|GetItemType))
  (return (== (Class|FGInventoryComponent|GetNumItems (Class|FGBuildableStorage|GetStorageInventory RequestStation) _itemtype) 0) _itemtype))

(fn GetAvailableItems
  (params (ProviderStation :type BP%20Provider%20Station%20Object%20Reference) (itemClass :type FG%20Item%20Descriptor%20Class%20Reference))
  (return (Class|FGInventoryComponent|GetNumItems (Class|FGBuildableStorage|GetStorageInventory ProviderStation) itemClass)))

(fn CreateOrder
  (params (ProviderStation :type BP%20Provider%20Station%20Object%20Reference) (RequestStation :type BP%20Request%20Station%20Object%20Reference) (ItemType :type FG%20Item%20Descriptor%20Class%20Reference))
  (bind _returnvalue (Class|FGBuildableStorage|GetStorageInventory ProviderStation))
  (bind (_out_stack _returnvalue_2) (Class|FGInventoryComponent|GetStackfromIndex _returnvalue))
  (if _returnvalue_2
    (Class|FGInventoryComponent|RemoveAllfromIndex _returnvalue)
    (bind _returnvalue_3 (Class|FGInventoryComponent|AddStack (Class|FGBuildableStorage|GetStorageInventory RequestStation) _out_stack false)) ; This just teleports the items to the Request Station without delay
    (Class|BlueprintLoggingLibrary|LogDisplay (Utilities|String|ToString(Text) (Utilities|Text|FormatText "Creating Order of {num} {type}." _returnvalue_3 (Class|FGItemDescriptor|GetItemName (.out_itemClass (Class|FGInventoryLibrary|BreakInventoryItem (.out_item (Class|FGInventoryLibrary|BreakInventoryStack _out_stack))))))))
    (return true)
    (else
      (return false))))